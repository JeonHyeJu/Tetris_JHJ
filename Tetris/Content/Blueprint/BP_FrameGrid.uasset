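; BP_FrameGrid is an actor that builds a U-shaped frame of instanced static meshes in the YZ plane, open at the top.
; Its Construction Script makes Cols odd, then lays a bottom row centred on the origin, spaced by Radius.
; It raises both side columns to Rows height, but those loops are nested, so column instances are added repeatedly at the same positions.
; The event graph is empty.
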(event EventBeginPlay)

(event Collision|EventActorBeginOverlap
  (params (OtherActor :type Actor%20Object%20Reference)))

(event EventTick
  (params (DeltaSeconds :type Float%20%28single-precision%29)))

(fn ConstructionScript
  (if (== (Math|Integer|%(Integer) (Variables|Default|GetCols) 2) 0)
    (Variables|Default|SetCols (+ (Variables|Default|GetCols) 1)))
  (Variables|Default|SetHalfCols (Math|Float|Ceil (/ (Variables|Default|GetCols) (Math|Float|MakeLiteralFloat 2.0))))
  (for _index (range (* (Variables|Default|GetHalfCols) -1) (Variables|Default|GetHalfCols))
    (Components|InstancedStaticMesh|AddInstance (Variables|Default|GetInstancedStaticMesh) (Math|Transform|MakeTransform (Math|Vector|MakeVector 0.0 (* _index (Variables|Default|GetRadius)) 0.0)) false)
    (for _index_2 (range 1 (Variables|Default|GetRows))
      (Components|InstancedStaticMesh|AddInstance (Variables|Default|GetInstancedStaticMesh) (Math|Transform|MakeTransform (Math|Vector|MakeVector 0.0 (* (Variables|Default|GetRadius) (* (Variables|Default|GetHalfCols) -1)) (* (Variables|Default|GetRadius) _index_2))) false)
      (for _index_3 (range 1 (Variables|Default|GetRows))
        (Components|InstancedStaticMesh|AddInstance (Variables|Default|GetInstancedStaticMesh) (Math|Transform|MakeTransform (Math|Vector|MakeVector 0.0 (* (Variables|Default|GetRadius) (Variables|Default|GetHalfCols)) (* _index_3 (Variables|Default|GetRadius)))) false)))))